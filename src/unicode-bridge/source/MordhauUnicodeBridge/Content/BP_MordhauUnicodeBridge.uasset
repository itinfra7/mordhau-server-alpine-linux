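; Server-side bridge actor for Mordhau that broadcasts Unicode chat messages to players through an RCON command.
; On BeginPlay it hooks the game mode's RCON string command event and listens for "unicode.say" followed by a numeric ID.
; The ID selects a pre-written .utf8 file, whose text reaches every player controller by calling ClientReceiveMessage by name.
; A successful file load also sends an ok reply to the requesting RCON client.
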(event `self.ReceiveBeginPlay`
  (bind _asmordhau_game_mode (cast `MordhauGameMode` (`GameplayStatics.GetGameMode`)))
  (add `MordhauGameMode.OnRconStringCommand` _asmordhau_game_mode (delegate `HandleUnicodeRconCommand`)))

(event `HandleUnicodeRconCommand`
  (params (Payload :type String) (ClientId :type Integer))
  (bind _returnvalue (`KismetStringLibrary.RightChop` Payload 12))
  (if (`KismetStringLibrary.StartsWith` Payload "unicode.say " "CaseSensitive")
    (if (`KismetStringLibrary.IsNumeric` _returnvalue)
      (bind (_loadedstring _returnvalue_2) (`MordhauUtilityLibrary.LoadStringFromFile` (`KismetStringLibrary.Concat_StrStr` "mordhau-unicode-bridge-" _returnvalue) ".utf8"))
      (if _returnvalue_2
        (bind _outactors (`GameplayStatics.GetAllActorsOfClass` "/Script/Mordhau.MordhauPlayerController"))
        (for _array_element _outactors
          (`MordhauUtilityLibrary.CallFunctionByNameWithArgs` (`KismetStringLibrary.Concat_StrStr` "ClientReceiveMessage " _loadedstring) _array_element))
        (`MordhauUtilityLibrary.SendMessageToRconClients` "unicode.say ok" ClientId)))))

(fn `UserConstructionScript`)